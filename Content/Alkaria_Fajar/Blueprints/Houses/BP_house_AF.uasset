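; BP_house_AF is a configurable house building for the Alkaria_Fajar location, set up entirely in its construction script.
; After running the parent script, it picks one of two facade meshes and one of two exterior materials from the Fasade and Finish enums.
; Mirrored flips the facade by negative Y scale, Mobility is applied to the mesh, and a text render shows an "AF" variant code.
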(fn `UserConstructionScript`
  (`parent.UserConstructionScript`)
  (`StaticMeshComponent.SetStaticMesh` (`self.sm_fasade`) (select `/Game/Alkaria_Fajar/Blueprints/Enumerations/enum_house_fasade` (`self.Fasade`) :`NewEnumerator0` "/Game/Alkaria_Fajar/Geometries/Raw/SM_AF1.SM_AF1" :`NewEnumerator1` "/Game/Alkaria_Fajar/Geometries/Raw/SM_AF2.SM_AF2" :!type "StaticMesh Object Reference"))
  (`SceneComponent.SetRelativeScale3D` (`self.sm_fasade`) (`KismetMathLibrary.MakeVector` 1.0 (select `bool` (`self.Mirrored`) :`false` 1.0 :`true` -1.0) 1.0))
  (`TextRenderComponent.K2_SetText` (`self.TextRender`) (`KismetTextLibrary.Conv_StringToText` (`KismetStringLibrary.Concat_StrStr` "AF" "" (`|GetEnumeratorNameAsString` (`self.Fasade`)) (`|GetEnumeratorNameAsString` (`self.Finish`)))))
  (`SceneComponent.SetMobility` (`self.sm_fasade`) (`self.Mobility`))
  (`PrimitiveComponent.SetMaterial` (`self.sm_fasade`) 0 (select `/Game/Alkaria_Fajar/Blueprints/Enumerations/enum_house_finish` (`self.Finish`) :`NewEnumerator0` "/Game/Alkaria_Fajar/Materials/MI_WAT_exterior_fasadeA.MI_WAT_exterior_fasadeA" :`NewEnumerator1` "/Game/Alkaria_Fajar/Materials/MI_WAT_exterior_fasadeB.MI_WAT_exterior_fasadeB" :!type "MaterialInterface Object Reference")))